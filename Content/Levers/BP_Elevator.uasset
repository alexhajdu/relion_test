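; BP_Elevator is a replicated elevator that lowers while an interaction is held and rises when it ends.
; Interface events InteractStart and InteractEnd set IsUp on the authority only.
; The IsUp RepNotify calls ElevatorUp or ElevatorDown, so movement follows replicated state rather than replicated transforms.
; A single Timeline drives the static mesh's relative Z, playing to descend and reversing from the end to rise.
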(event Custom|ElevatorUp
  (bind _newtrack_0 (Timeline|Timeline ReverseFromEnd)
    (:Update
      (Transformation|SetRelativeLocation (Variables|Default|GetStaticMesh) (Math|Vector|MakeVector 0.0 0.0 (* _newtrack_0 -1e+02)) false false))))

(event Custom|ElevatorDown
  (bind _newtrack_0 (Timeline|Timeline Play)
    (:Update
      (Transformation|SetRelativeLocation (Variables|Default|GetStaticMesh) (Math|Vector|MakeVector 0.0 0.0 (* _newtrack_0 -1e+02)) false false))))

(event EventBeginPlay)

(event EventInteractStart
  (params (Interactor :type Actor%20Object%20Reference))
  ;[0.15 0.15 0.15 0.5] Interface
  (Networking|SwitchHasAuthority
    (:Authority
      (Variables|Default|SetisUp false))))

(event EventInteractEnd
  (params (Interactor :type Actor%20Object%20Reference))
  ;[0.15 0.15 0.15 0.5] Interface
  (Networking|SwitchHasAuthority
    (:Authority
      (Variables|Default|SetisUp true))))

(fn ConstructionScript)

(fn OnRepIsUp
  (if (Variables|Default|GetisUp)
    (CallFunction|ElevatorUp)
    (else
      (CallFunction|ElevatorDown))))